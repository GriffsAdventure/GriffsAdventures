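; Door_BP is a double-leaf ancient door that swings open when its OpenAncientDoor event is called.
; The event plays the Ancient_Door sound at the root's location and starts the DoorRotation timeline.
; The timeline's DoorOpen track drives both leaves' yaw: RightDoor in relative space, LeftDoor in world space with a hardcoded mirrored offset, tying it to the actor's placed orientation.
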(event `Open Ancient Door`
  (`GameplayStatics.SpawnSoundAtLocation` "/Game/Carlos/Ancient_Door.Ancient_Door" (`SceneComponent.K2_GetComponentLocation` (`self.DefaultSceneRoot`)))
  (bind (_direction _dooropen) (`Timeline|DoorRotation`)
    (:`Update`
      (`|ExecutionSequence`
        (:`then_0`
          (`SceneComponent.K2_SetRelativeRotation` (`self.Right_Door`) (`KismetMathLibrary.MakeRotator` 0.0 0.0 _dooropen) false false))
        (:`then_1`
          (`SceneComponent.K2_SetWorldRotation` (`self.Left_Door`) (`KismetMathLibrary.MakeRotator` 0.0 0.0 (- 200.0 _dooropen)) false false))))))

(fn `UserConstructionScript`)
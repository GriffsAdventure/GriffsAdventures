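; Target indicator circle whose look reflects the player's current target type.
; On BeginPlay, a brief delay precedes reading the ThirdPersonCharacter's friendly and enemy flags to set a green or red material.
; A downward line trace immediately moves the circle mesh to the hit actor's location, without checking for a hit.
; A slightly later delayed step doubles the circle's scale for boss targets, reusing the earlier character cast.
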(event `self.ReceiveBeginPlay`
  (bind _interactive_circle (`self.Interactive Circle`))
  (bind _interactive_circle_2 (`self.Interactive Circle`))
  (bind _returnvalue (`SceneComponent.K2_GetComponentLocation` _interactive_circle))
  ;[1 1 1] Sets the material of the circle
  (`|ExecutionSequence`
    (:`then_0`
      (`KismetSystemLibrary.Delay` 0.03)
      (bind _asthird_person_character (cast `/Game/Character/Blueprints/ThirdPersonCharacter` (`GameplayStatics.GetPlayerCharacter` 0)))
      (`|ExecutionSequence`
        (:`then_0`
          (if (`/Game/Character/Blueprints/ThirdPersonCharacter.FriendlyTarget?` _asthird_person_character)
            (`PrimitiveComponent.SetMaterial` _interactive_circle_2 0 "/Game/Leigh/UI/Models/Materials/M_PaleGreen.M_PaleGreen")))
        (:`then_1`
          (if (`/Game/Character/Blueprints/ThirdPersonCharacter.EnemyTarget?` _asthird_person_character)
            (`PrimitiveComponent.SetMaterial` _interactive_circle_2 0 "/Game/Leigh/UI/Models/Materials/M_Red.M_Red")))))
    (:`then_1`
      (bind _outhit (`KismetSystemLibrary.LineTraceSingle` _returnvalue (+ _returnvalue (`KismetMathLibrary.MakeVector` 0.0 0.0 -600.0)) "TraceTypeQuery1"))
      (`SceneComponent.K2_SetWorldLocation` _interactive_circle (`self.K2_GetActorLocation` (`.HitActor` (`GameplayStatics.BreakHitResult` _outhit))) false false))
    (:`then_2`
      (`KismetSystemLibrary.Delay` 0.04)
      (if (`/Game/Character/Blueprints/ThirdPersonCharacter.BossTarget?` _asthird_person_character)
        (`SceneComponent.SetRelativeScale3D` _interactive_circle (* (`SceneComponent.RelativeScale3D` _interactive_circle) 2.0))))))

(fn `UserConstructionScript`)
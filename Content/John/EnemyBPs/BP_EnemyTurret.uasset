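; Enemy turret that turns to face the player when PawnSensing sees them and launches BP_Projectile by impulse, throttled by a delay.
; DoDamage subtracts the attacking player's AttackDamage from BotHealth and blinks the cube material.
; Tick maps BotHealth to ten health-bar components via per-value visibility functions and destroys the turret at zero.
; SpawnOutline opens a Tick-fed gate that shows a highlight outline while the player's EnemyTargeted flag is set.
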(event `SpawnOutline`
  (bind _outline (`self.Outline`))
  ;[0 0.3573 1] Spawns Outline
  (goto _label :!via `Open`))

(event `self.ReceiveTick`
  (params (DeltaSeconds :type "Float (single-precision)"))
  (bind _outline (`self.Outline`))
  (`|ExecutionSequence`
    (:`then_0`
      ;[0 0.3573 1] Sets the healthbar of enemy
      (switch `int` (`self.Bot_Health`)
        (:`1`
          (`SceneComponent.SetVisibility` (`self.Health01`) true false)
          (`SceneComponent.SetVisibility` (`self.Health02`) false false)
          (`SceneComponent.SetVisibility` (`self.Health03`) false false)
          (`SceneComponent.SetVisibility` (`self.Health04`) false false)
          (`SceneComponent.SetVisibility` (`self.Health05`) false false)
          (`SceneComponent.SetVisibility` (`self.Health06`) false false)
          (`SceneComponent.SetVisibility` (`self.Health07`) false false)
          (`SceneComponent.SetVisibility` (`self.Health08`) false false)
          (`SceneComponent.SetVisibility` (`self.Health09`) false false)
          (`SceneComponent.SetVisibility` (`self.Health10`) false false))
        (:`2`
          (`SceneComponent.SetVisibility` (`self.Health01`) true false)
          (`SceneComponent.SetVisibility` (`self.Health02`) true false)
          (`SceneComponent.SetVisibility` (`self.Health03`) false false)
          (`SceneComponent.SetVisibility` (`self.Health04`) false false)
          (`SceneComponent.SetVisibility` (`self.Health05`) false false)
          (`SceneComponent.SetVisibility` (`self.Health06`) false false)
          (`SceneComponent.SetVisibility` (`self.Health07`) false false)
          (`SceneComponent.SetVisibility` (`self.Health08`) false false)
          (`SceneComponent.SetVisibility` (`self.Health09`) false false)
          (`SceneComponent.SetVisibility` (`self.Health10`) false false))
        (:`3`
          (`SceneComponent.SetVisibility` (`self.Health01`) true false)
          (`SceneComponent.SetVisibility` (`self.Health02`) true false)
          (`SceneComponent.SetVisibility` (`self.Health03`) true false)
          (`SceneComponent.SetVisibility` (`self.Health10`) false false)
          (`SceneComponent.SetVisibility` (`self.Health09`) false false)
          (`SceneComponent.SetVisibility` (`self.Health08`) false false)
          (`SceneComponent.SetVisibility` (`self.Health07`) false false)
          (`SceneComponent.SetVisibility` (`self.Health06`) false false)
          (`SceneComponent.SetVisibility` (`self.Health05`) false false)
          (`SceneComponent.SetVisibility` (`self.Health04`) false false))
        (:`4`
          (`SceneComponent.SetVisibility` (`self.Health01`) true false)
          (`SceneComponent.SetVisibility` (`self.Health02`) true false)
          (`SceneComponent.SetVisibility` (`self.Health03`) true false)
          (`SceneComponent.SetVisibility` (`self.Health04`) true false)
          (`SceneComponent.SetVisibility` (`self.Health10`) false false)
          (`SceneComponent.SetVisibility` (`self.Health09`) false false)
          (`SceneComponent.SetVisibility` (`self.Health08`) false false)
          (`SceneComponent.SetVisibility` (`self.Health07`) false false)
          (`SceneComponent.SetVisibility` (`self.Health06`) false false)
          (`SceneComponent.SetVisibility` (`self.Health05`) false false))
        (:`5`
          (`SceneComponent.SetVisibility` (`self.Health01`) true false)
          (`SceneComponent.SetVisibility` (`self.Health02`) true false)
          (`SceneComponent.SetVisibility` (`self.Health03`) true false)
          (`SceneComponent.SetVisibility` (`self.Health04`) true false)
          (`SceneComponent.SetVisibility` (`self.Health05`) true false)
          (`SceneComponent.SetVisibility` (`self.Health10`) false false)
          (`SceneComponent.SetVisibility` (`self.Health09`) false false)
          (`SceneComponent.SetVisibility` (`self.Health08`) false false)
          (`SceneComponent.SetVisibility` (`self.Health07`) false false)
          (`SceneComponent.SetVisibility` (`self.Health06`) false false))
        (:`6`
          (`SceneComponent.SetVisibility` (`self.Health01`) true false)
          (`SceneComponent.SetVisibility` (`self.Health02`) true false)
          (`SceneComponent.SetVisibility` (`self.Health03`) true false)
          (`SceneComponent.SetVisibility` (`self.Health04`) true false)
          (`SceneComponent.SetVisibility` (`self.Health05`) true false)
          (`SceneComponent.SetVisibility` (`self.Health06`) true false)
          (`SceneComponent.SetVisibility` (`self.Health10`) false false)
          (`SceneComponent.SetVisibility` (`self.Health08`) false false)
          (`SceneComponent.SetVisibility` (`self.Health07`) false false)
          (`SceneComponent.SetVisibility` (`self.Health09`) false false))
        (:`7`
          (`SceneComponent.SetVisibility` (`self.Health01`) true false)
          (`SceneComponent.SetVisibility` (`self.Health02`) true false)
          (`SceneComponent.SetVisibility` (`self.Health03`) true false)
          (`SceneComponent.SetVisibility` (`self.Health04`) true false)
          (`SceneComponent.SetVisibility` (`self.Health05`) true false)
          (`SceneComponent.SetVisibility` (`self.Health06`) true false)
          (`SceneComponent.SetVisibility` (`self.Health07`) true false)
          (`SceneComponent.SetVisibility` (`self.Health10`) false false)
          (`SceneComponent.SetVisibility` (`self.Health09`) false false)
          (`SceneComponent.SetVisibility` (`self.Health08`) false false))
        (:`8`
          (`SceneComponent.SetVisibility` (`self.Health01`) true false)
          (`SceneComponent.SetVisibility` (`self.Health02`) true false)
          (`SceneComponent.SetVisibility` (`self.Health03`) true false)
          (`SceneComponent.SetVisibility` (`self.Health04`) true false)
          (`SceneComponent.SetVisibility` (`self.Health05`) true false)
          (`SceneComponent.SetVisibility` (`self.Health06`) true false)
          (`SceneComponent.SetVisibility` (`self.Health07`) true false)
          (`SceneComponent.SetVisibility` (`self.Health08`) true false)
          (`SceneComponent.SetVisibility` (`self.Health10`) false false)
          (`SceneComponent.SetVisibility` (`self.Health09`) false false))
        (:`9`
          (`SceneComponent.SetVisibility` (`self.Health01`) true false)
          (`SceneComponent.SetVisibility` (`self.Health02`) true false)
          (`SceneComponent.SetVisibility` (`self.Health03`) true false)
          (`SceneComponent.SetVisibility` (`self.Health04`) true false)
          (`SceneComponent.SetVisibility` (`self.Health05`) true false)
          (`SceneComponent.SetVisibility` (`self.Health06`) true false)
          (`SceneComponent.SetVisibility` (`self.Health07`) true false)
          (`SceneComponent.SetVisibility` (`self.Health08`) true false)
          (`SceneComponent.SetVisibility` (`self.Health09`) true false)
          (`SceneComponent.SetVisibility` (`self.Health10`) false false))
        (:`10`
          (`SceneComponent.SetVisibility` (`self.Health01`) true false)
          (`SceneComponent.SetVisibility` (`self.Health02`) true false)
          (`SceneComponent.SetVisibility` (`self.Health03`) true false)
          (`SceneComponent.SetVisibility` (`self.Health04`) true false)
          (`SceneComponent.SetVisibility` (`self.Health05`) true false)
          (`SceneComponent.SetVisibility` (`self.Health06`) true false)
          (`SceneComponent.SetVisibility` (`self.Health07`) true false)
          (`SceneComponent.SetVisibility` (`self.Health08`) true false)
          (`SceneComponent.SetVisibility` (`self.Health09`) true false)
          (`SceneComponent.SetVisibility` (`self.Health10`) true false))))
    (:`then_1`
      ;[0 0.3573 1] Spawns Outline
      (`/Engine/EditorBlueprintResources/StandardMacros.Gate` true :!label _label
        (:`Exit`
          (bind _asthird_person_character (cast `/Game/Character/Blueprints/ThirdPersonCharacter` (`GameplayStatics.GetPlayerCharacter` 0) :!label _label_2))
          (if (`/Game/Character/Blueprints/ThirdPersonCharacter.EnemyTargeted` _asthird_person_character)
            (`|ExecutionSequence`
              (:`then_0`
                (`/Engine/EditorBlueprintResources/StandardMacros.DoOnce` false :!label _label_3
                  (:`Completed`
                    (`PrimitiveComponent.SetMaterial` _outline 0 "/Game/David/Interactive_Mat.Interactive_Mat")
                    (`SceneComponent.SetHiddenInGame` _outline false false)
                    (goto _label_4 :!via `Reset`))))
              (:`then_1`
                (`KismetSystemLibrary.Delay` 0.01)
                (goto _label_2)))
            (else
              (`/Engine/EditorBlueprintResources/StandardMacros.DoOnce` false :!label _label_4
                (:`Completed`
                  (`SceneComponent.SetHiddenInGame` _outline true false)
                  (`|ExecutionSequence`
                    (:`then_0`
                      (goto _label_3 :!via `Reset`))
                    (:`then_1`
                      (goto _label :!via `Close`))))))))))
    (:`then_2`
      ;[0 0.3573 1] Sudden Death
      (if (<= (`self.Bot_Health`) 0)
        (`self.K2_DestroyActor`)))))

(event `DamageTaken`
  ;[0 0.3573 1] Spawns Outline
)

(event `DoDamage`
  (bind _cube (`self.Cube`))
  (bind _blinkduration (`self.BlinkDuration`))
  (bind _timesblinked (`self.TimesBlinked`))
  ;[0 0.3573 1] Bot Takes Damage
  (bind _asthird_person_character (cast `/Game/Character/Blueprints/ThirdPersonCharacter` (`GameplayStatics.GetPlayerCharacter` 0)))
  (if (`/Game/Character/Blueprints/ThirdPersonCharacter.HasAttacked?` _asthird_person_character)
    (set `self.Bot_Health` (- (`self.Bot_Health`) (`/Game/Character/Blueprints/ThirdPersonCharacter.AttackDamage` _asthird_person_character)))
    (`PrimitiveComponent.SetMaterial` _cube 0 "/Game/David/Interactive_Mat.Interactive_Mat" :!label _label_5)
    (`KismetSystemLibrary.Delay` _blinkduration)
    (`PrimitiveComponent.SetMaterial` _cube 0 "/Game/Maps/Geometry/Meshes/CubeMaterial.CubeMaterial")
    (`KismetSystemLibrary.Delay` _blinkduration)
    (set `self.TimesBlinked` (+ _timesblinked 1))
    (if (== _timesblinked (`self.DMGTakenFlashes`))
      (set `self.TimesBlinked` 0)
      (else
        (goto _label_5)))))

(event `self.PawnSensing.OnSeePawn`
  (params (Pawn :type "Pawn Object Reference"))
  (bind _asthird_person_character (cast `/Game/Character/Blueprints/ThirdPersonCharacter` Pawn))
  (`|ExecutionSequence`
    (:`then_0`
      (`self.K2_SetActorRotation` (`KismetMathLibrary.FindLookAtRotation` (`self.K2_GetActorLocation`) (`self.K2_GetActorLocation` _asthird_person_character))))
    (:`then_1`
      (if (`self.SpawnProjectile`)
        (bind _returnvalue (`|SpawnActorFromClass` "/Game/John/BP_Projectile.BP_Projectile_C" (`SceneComponent.K2_GetComponentToWorld` (`self.ProjectSpawnLocation`)) "Undefined" "OverrideRootScale" null null))
        (`PrimitiveComponent.AddImpulse` (`/Game/John/BP_Projectile.Sphere` _returnvalue) (* (`SceneComponent.GetForwardVector` (`self.Cube`)) (`self.ShootAmount`)) "None" false)
        (set `self.SpawnProjectile` false)
        (`KismetSystemLibrary.Delay` 1.5)
        (set `self.SpawnProjectile` true)))))

(fn `UserConstructionScript`)